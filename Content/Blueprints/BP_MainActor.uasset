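; Main input actor that flies the level's CameraActor and controls an SWS actor, both found on BeginPlay.
; Axis mappings move the camera along forward, right and world Z, and holding right mouse enables free look.
; The mouse wheel zooms by scaling camera location relative to world origin, and Enter restores the default view.
; Input actions toggle SWS Stop/Play through a FlipFlop (Stop first), call Step, or quit the game.
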(event `self.ReceiveBeginPlay`
  (bind _returnvalue (`GameplayStatics.GetActorOfClass` "/Script/Engine.CameraActor"))
  (set `self.Camera` _returnvalue)
  (bind _returnvalue_2 (`GameplayStatics.GetActorOfClass` "/Script/SWS.SWS"))
  (set `self.SWS` _returnvalue_2))

(event `InputAction|ActionTogglePlayPause`
  (params (Key :type "Key Structure"))
  (bind _sws (`self.SWS`))
  (:`Pressed`
    (`/Engine/EditorBlueprintResources/StandardMacros.FlipFlop`
      (:`A`
        (`SWS.Stop` _sws))
      (:`B`
        (`SWS.Play` _sws)))))

(event `InputAxis|XAxisMapping`
  (params (AxisValue :type "Float (single-precision)"))
  (bind _camera (`self.Camera`))
  ;[1 1 1] Move Camera Forward
  (`self.K2_SetActorLocation` _camera (+ (`self.K2_GetActorLocation` _camera) (* (`KismetMathLibrary.GetForwardVector` (`self.K2_GetActorRotation` _camera)) (* AxisValue (`self.Speed`)))) false false))

(event `Key|MouseScrollDown`
  (params (Key :type "Key Structure"))
  (bind _camera (`self.Camera`))
  ;[1 1 1] Mouse Wheel Zoom Out
  (:`Pressed`
    (`self.K2_SetActorLocation` _camera (* (`self.K2_GetActorLocation` _camera) (1.3 1.3 1.3)) false false)))

(event `InputAxis|XAxisMappingNegative`
  (params (AxisValue :type "Float (single-precision)"))
  (bind _camera (`self.Camera`))
  ;[1 1 1] Move Camera Backward
  (`self.K2_SetActorLocation` _camera (+ (`self.K2_GetActorLocation` _camera) (* (`KismetMathLibrary.GetForwardVector` (`self.K2_GetActorRotation` _camera)) (* AxisValue (`self.Speed`)))) false false))

(event `Key|MouseScrollUp`
  (params (Key :type "Key Structure"))
  (bind _camera (`self.Camera`))
  ;[1 1 1] Mouse Wheel Zoom In
  (:`Pressed`
    (`self.K2_SetActorLocation` _camera (* (`self.K2_GetActorLocation` _camera) (0.7 0.7 0.7)) false false)))

(event `InputAxis|YAxisMapping`
  (params (AxisValue :type "Float (single-precision)"))
  (bind _camera (`self.Camera`))
  ;[1 1 1] Move Camera Left
  (`self.K2_SetActorLocation` _camera (+ (`self.K2_GetActorLocation` _camera) (* (`KismetMathLibrary.GetRightVector` (`self.K2_GetActorRotation` _camera)) (* AxisValue (`self.Speed`)))) false false))

(event `Key|RightMouseButton`
  (params (Key :type "Key Structure"))
  (bind _returnvalue (`GameplayStatics.GetPlayerController` 0))
  ;[1 1 1] Enter and Leave FreeLook Mode
  (:`Pressed`
    (set `self.DoFreeLook` true)
    (set `PlayerController.bShowMouseCursor` false _returnvalue))
  (:`Released`
    (set `self.DoFreeLook` false)
    (set `PlayerController.bShowMouseCursor` true _returnvalue)))

(event `InputAxisKey|MouseX`
  (params (AxisValue :type "Float (single-precision)"))
  (bind _camera (`self.Camera`))
  (bind (_returnvalue_roll _returnvalue_pitch _returnvalue_yaw) (`KismetMathLibrary.BreakRotator` (`self.K2_GetActorRotation` _camera)))
  ;[1 1 1] MouseFreeLook X Coord
  (if (`self.DoFreeLook`)
    (`self.K2_SetActorRotation` _camera (`KismetMathLibrary.MakeRotator` _returnvalue_roll _returnvalue_pitch (+ _returnvalue_yaw AxisValue)) false)))

(event `InputAxis|YAxisMappingNegative`
  (params (AxisValue :type "Float (single-precision)"))
  (bind _camera (`self.Camera`))
  ;[1 1 1] Move Camera Right
  (`self.K2_SetActorLocation` _camera (+ (`self.K2_GetActorLocation` _camera) (* (`KismetMathLibrary.GetRightVector` (`self.K2_GetActorRotation` _camera)) (* AxisValue (`self.Speed`)))) false false))

(event `InputAxisKey|MouseY`
  (params (AxisValue :type "Float (single-precision)"))
  (bind _camera (`self.Camera`))
  (bind (_returnvalue_roll _returnvalue_pitch _returnvalue_yaw) (`KismetMathLibrary.BreakRotator` (`self.K2_GetActorRotation` _camera)))
  ;[1 1 1] MouseFreeLook Y Coord
  (if (`self.DoFreeLook`)
    (`self.K2_SetActorRotation` _camera (`KismetMathLibrary.MakeRotator` _returnvalue_roll (+ _returnvalue_pitch AxisValue) _returnvalue_yaw) false)))

(event `InputAxis|ZAxisMapping`
  (params (AxisValue :type "Float (single-precision)"))
  (bind _camera (`self.Camera`))
  ;[1 1 1] Move Camera Up
  (`self.K2_SetActorLocation` _camera (+ (`self.K2_GetActorLocation` _camera) (`KismetMathLibrary.MakeVector` 0.0 0.0 (* AxisValue (`self.Speed`)))) false false))

(event `Key|Enter`
  (params (Key :type "Key Structure"))
  ;[1 1 1] SetDefaultCameraView
  (:`Pressed`
    (`self.K2_SetActorLocationAndRotation` (`self.Camera`) (`self.CameraDefaultLocation`) (`self.CameraDefaultRotation`) false false)))

(event `InputAxis|ZAxisMappingNegative`
  (params (AxisValue :type "Float (single-precision)"))
  (bind _camera (`self.Camera`))
  ;[1 1 1] Move Camera Down
  (`self.K2_SetActorLocation` _camera (+ (`self.K2_GetActorLocation` _camera) (`KismetMathLibrary.MakeVector` 0.0 0.0 (* AxisValue (`self.Speed`)))) false false))

(event `InputAction|ActionExit`
  (params (Key :type "Key Structure"))
  (:`Pressed`
    (`KismetSystemLibrary.QuitGame` null "Quit")))

(event `InputAction|ActionStep`
  (params (Key :type "Key Structure"))
  (:`Pressed`
    (`SWS.Step` (`self.SWS`))))

(fn `UserConstructionScript`)