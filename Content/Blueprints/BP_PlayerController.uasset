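; Player controller that lets the player click bodies in the SWS world to select and inspect them.
; On BeginPlay it shows the cursor, adds the controls HUD and a hidden body-info widget, and finds the SWS actor.
; Left click clears the world's selection, then a cursor trace selects any hit TheBody component by index and displays its name, mass and size.
; A click hitting nothing hides the info panel.
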(event `self.ReceiveBeginPlay`
  (bind _returnvalue (`|CreateWidget` "/Game/HUD/WB_BodyInfo.WB_BodyInfo_C"))
  (`UserWidget.AddToViewport` _returnvalue 0)
  (`Widget.SetVisibility` _returnvalue "Hidden")
  (set `self.BodyInfoWidget` _returnvalue)
  (set `self.bShowMouseCursor` true)
  (bind _returnvalue_2 (`|CreateWidget` "/Game/HUD/HUD_Controls.HUD_Controls_C"))
  (`UserWidget.AddToViewport` _returnvalue_2 0)
  (bind _returnvalue_3 (`GameplayStatics.GetActorOfClass` "/Script/SWS.SWS"))
  (set `self.World` _returnvalue_3))

(event `Key|LeftMouseButton`
  (params (Key :type "Key Structure"))
  (bind _bodyinfowidget (`self.BodyInfoWidget`))
  (bind (_hitresult _returnvalue) (`self.GetHitResultUnderCursorByChannel` (`GameplayStatics.GetPlayerController` 0) "TraceTypeQuery1" true))
  (bind (_bblockinghit _binitialoverlap _time _distance _location _impactpoint _normal _impactnormal _physmat _hitactor _hitcomponent) (`GameplayStatics.BreakHitResult` _hitresult))
  (:`Pressed`
    (`SWS.DeselectBodies` (`self.World`))
    (if _returnvalue
      (if (`KismetMathLibrary.ClassIsChildOf` (`GameplayStatics.GetObjectClass` _hitcomponent) "/Script/SWS.TheBody")
        (bind _asthe_body (cast `TheBody` _hitcomponent))
        (bind _output_get (set `self.SelectedBody` _asthe_body))
        (`Widget.SetVisibility` _bodyinfowidget "Visible")
        (`TextBlock.SetText` (`/Game/HUD/WB_BodyInfo.TB_BodyName` _bodyinfowidget) (`KismetTextLibrary.Conv_StringToText` (`TheBody.BodyName` _output_get)))
        (`TextBlock.SetText` (`/Game/HUD/WB_BodyInfo.TB_BodyMass` _bodyinfowidget) (`KismetTextLibrary.Conv_DoubleToText` (`TheBody.m` _output_get) "HalfToEven"))
        (`TextBlock.SetText` (`/Game/HUD/WB_BodyInfo.TB_BodySize` _bodyinfowidget) (`KismetTextLibrary.Conv_DoubleToText` (`TheBody.s` _output_get) "HalfToEven"))
        (`SWS.SetBodySelected` (`self.World`) (`TheBody.index` _output_get) true))
      (else
        (set `self.SelectedBody` null)
        (`Widget.SetVisibility` _bodyinfowidget "Hidden")))))

(fn `UserConstructionScript`)